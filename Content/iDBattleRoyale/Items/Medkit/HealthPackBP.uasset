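; HealthPackBP is a medkit pickup that adds health to the player.
; A timeline started at BeginPlay drives the yaw of the Medkit component to spin it.
; Any actor overlap adds HealthAddition to the Health of player 0's Battle_Royale_Player character, without checking which actor overlapped or clamping the result, then destroys the pickup if that cast succeeded.
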(event Collision|EventActorBeginOverlap
  (params (OtherActor :type Actor%20Object%20Reference))
  (bind _asbattle_royale_player (Utilities|Casting|CastToBattle_Royale_Player (Game|GetPlayerCharacter 0)))
  (Variables|/Game/iDBattleRoyale/PlayerCharacter/Battle_Royale_Player.Battle_Royale_Player_C|SetHealth _asbattle_royale_player (+ (Variables|/Game/iDBattleRoyale/PlayerCharacter/Battle_Royale_Player.Battle_Royale_Player_C|GetHealth _asbattle_royale_player) (Variables|Default|GetHealth%20Addition)))
  (Actor|DestroyActor))

(event EventBeginPlay
  (bind _newtrack_0 (Timeline|Timeline_0 Play)
    (:Update
      (Transformation|SetRelativeRotation (Variables|Default|Getmedkit) (Math|Rotator|MakeRotator 0.0 0.0 (* _newtrack_0 3.6e+02)) false false))))

(fn ConstructionScript)